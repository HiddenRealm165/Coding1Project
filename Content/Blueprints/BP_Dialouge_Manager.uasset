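; BP_Dialouge_Manager is an actor that shows timed dialogue lines on screen through a W_DialogueBox widget.
; On BeginPlay it creates and stores the widget.
; Each DisplayNextLine call sets the current Dialogue array entry as its text, shows it in the viewport for a five-second delay, then removes it and advances the index.
; The index wraps to the first line once it passes the end.
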(event `self.ReceiveBeginPlay`
  (bind _returnvalue (`|CreateWidget` "/Game/Widgets/W_DialogueBox.W_DialogueBox_C"))
  (set `self.WidgetDialogue` _returnvalue))

(event `self.ReceiveActorBeginOverlap`
  (params (OtherActor :type "Actor Object Reference")))

(event `DisplayNextLine`
  (bind _widgetdialogue (`self.WidgetDialogue`))
  (if (>= (`self.DialogueIndex`) (`KismetArrayLibrary.Array_Length` (`self.Dialogue`)))
    (set `self.DialogueIndex` 0))
  (`/Game/Widgets/W_DialogueBox.SetNewText` (`self.WidgetDialogue`) (`|GetArrayItem` (`self.Dialogue`) (`self.DialogueIndex`)))
  (`UserWidget.AddToViewport` _widgetdialogue 0)
  (`KismetSystemLibrary.Delay` 5.0)
  (`Widget.RemoveFromParent` _widgetdialogue)
  (`/Engine/EditorBlueprintResources/StandardMacros.IncrementInt` (`self.DialogueIndex`)))

(fn `UserConstructionScript`)