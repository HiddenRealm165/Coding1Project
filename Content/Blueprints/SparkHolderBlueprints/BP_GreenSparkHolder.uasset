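; Actor that holds a green spark and, when the player character touches it, asks the green spark holder manager to bring a spark to it.
; It finds the manager on BeginPlay and tracks the spark inside its Box via overlap events, while Capsule overlaps by the player trigger RequestSpark.
; SendSparkToRequester teleports the held spark to a requesting holder's TeleportPoint with zero rotation.
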(event `self.ReceiveBeginPlay`
  (bind _returnvalue (`GameplayStatics.GetActorOfClass` "/Game/Blueprints/SparkHolderBlueprints/BP_GreenSparkHolderManager.BP_GreenSparkHolderManager_C"))
  (set `self.SparkHolderManager` _returnvalue))

(event `self.Box.OnComponentBeginOverlap`
  (params (OverlappedComponent :type "PrimitiveComponent Object Reference") (OtherActor :type "Actor Object Reference") (OtherComp :type "PrimitiveComponent Object Reference") (OtherBodyIndex :type Integer) (bFromSweep :type Boolean) (SweepResult :type "HitResult Structure (by ref)"))
  (bind _asbp_green_spark (cast `/Game/Blueprints/SparkTypes/BP_GreenSpark` OtherActor))
  (set `self.Spark` _asbp_green_spark))

(event `self.Box.OnComponentEndOverlap`
  (params (OverlappedComponent :type "PrimitiveComponent Object Reference") (OtherActor :type "Actor Object Reference") (OtherComp :type "PrimitiveComponent Object Reference") (OtherBodyIndex :type Integer))
  (if (== OtherActor (`self.Spark`))
    (set `self.Spark` null)))

(event `self.Capsule.OnComponentBeginOverlap`
  (params (OverlappedComponent :type "PrimitiveComponent Object Reference") (OtherActor :type "Actor Object Reference") (OtherComp :type "PrimitiveComponent Object Reference") (OtherBodyIndex :type Integer) (bFromSweep :type Boolean) (SweepResult :type "HitResult Structure (by ref)"))
  (cast `/Game/ThirdPerson/Blueprints/BP_ThirdPersonCharacter` OtherActor)
  (`/Game/Blueprints/SparkHolderBlueprints/BP_GreenSparkHolderManager.RequestSpark` (`self.SparkHolderManager`) self))

(event `SendSparkToRequester`
  (params (Requester :type "/Game/Blueprints/SparkHolderBlueprints/BP_GreenSparkHolder Object Reference"))
  (`self.K2_TeleportTo` :`self` (`self.Spark`) :`DestLocation` (`SceneComponent.K2_GetComponentLocation` (`/Game/Blueprints/SparkHolderBlueprints/BP_GreenSparkHolder.TeleportPoint` Requester))))

(fn `UserConstructionScript`)