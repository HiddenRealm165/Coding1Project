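; BP_Tree is a tree actor that grows in random steps after BeginPlay and takes on a random mesh.
; GrowLoop re-calls itself after random delays, capped by a DoN whose random limit is re-rolled on every call.
; Each Grow adds random scale to SMTree and enables collision once the scale passes a threshold.
; Only the first Grow swaps the mesh to a random pick from PossibleTreeMeshes.
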(event `self.ReceiveBeginPlay`
  (`self.GrowLoop` false))

(event `GrowLoop`
  (params (ResetLoop :type Boolean))
  (bind _output_get (set `self.GrowLoopAmount` (`KismetMathLibrary.RandomIntegerInRange` (`self.MinGrowLoopAmount`) (`self.MaxGrowLoopAmount`))))
  (`/Engine/EditorBlueprintResources/StandardMacros.Do N` _output_get
    (:`Exit`
      (`KismetSystemLibrary.Delay` (`KismetMathLibrary.RandomFloatInRange` 1.0 4.0))
      (`self.Grow`)
      (`self.GrowLoop` false))))

(event `Grow`
  (bind _sm_tree (`self.SM_Tree`))
  (bind _relativescale3d_x (`KismetMathLibrary.BreakVector` (`SceneComponent.RelativeScale3D` (`self.SM_Tree`))))
  (`SceneComponent.SetRelativeScale3D` _sm_tree (+ (`SceneComponent.RelativeScale3D` _sm_tree) (`KismetMathLibrary.RandomFloatInRange` 0.1 0.25)))
  (if (> _relativescale3d_x 0.4)
    (`PrimitiveComponent.SetCollisionEnabled` (`self.SM_Tree`) "QueryAndPhysics"))
  (`/Engine/EditorBlueprintResources/StandardMacros.DoOnce` false
    (:`Completed`
      (`self.ChangeToRandomTree`))))

(event `ChangeToRandomTree`
  (`StaticMeshComponent.SetStaticMesh` (`self.SM_Tree`) (`KismetArrayLibrary.Array_Random` (`self.possibleTreeMeshes`))))

(fn `UserConstructionScript`)