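; BP_Key is a key pickup that adds a key to the player's total when BP_ThirdPersonCharacter overlaps it.
; After calling AddKey on the character, it hides its static mesh and turns off collision instead of destroying itself.
; The SpawnKey event makes a hidden key visible again with query-only collision, so the same actor can be reused.
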(event `self.ReceiveBeginPlay`)

(event `self.ReceiveActorBeginOverlap`
  (params (OtherActor :type "Actor Object Reference"))
  (bind _staticmesh (`self.StaticMesh`))
  (bind _asbp_third_person_character (cast `/Game/ThirdPerson/Blueprints/BP_ThirdPersonCharacter` OtherActor))
  (`/Game/ThirdPerson/Blueprints/BP_ThirdPersonCharacter.AddKey` _asbp_third_person_character) ; Adds 1 key to TotalKeys on Player
  (`SceneComponent.SetVisibility` _staticmesh false false)
  (`PrimitiveComponent.SetCollisionEnabled` _staticmesh "NoCollision"))

(event `self.ReceiveTick`
  (params (DeltaSeconds :type "Float (single-precision)")))

(event `SpawnKey`
  (bind _staticmesh (`self.StaticMesh`))
  (if (not (`SceneComponent.IsVisible` _staticmesh))
    (`SceneComponent.SetVisibility` _staticmesh true false)
    (`PrimitiveComponent.SetCollisionEnabled` _staticmesh "QueryOnly")))

(fn `UserConstructionScript`)