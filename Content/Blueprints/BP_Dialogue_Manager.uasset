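; BP_Dialogue_Manager is an actor that queues dialogue lines and shows them one at a time in a W_DialogueBox widget created on BeginPlay.
; AddDialogueToQueue appends a line and starts display if nothing is showing.
; ProgressDialogue advances the index to the next line, or clears the queue and removes the widget after the last one.
; An older timed, looping display chain remains in the graph but is disconnected.
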(event `self.ReceiveBeginPlay`
  (bind _returnvalue (`|CreateWidget` "/Game/Widgets/W_DialogueBox.W_DialogueBox_C"))
  (set `self.WidgetDialogue` _returnvalue))

(event `self.ReceiveActorBeginOverlap`
  (params (OtherActor :type "Actor Object Reference")))

(event `DisplayNextLine`
  (set `self.IsDisplaying` true)
  (`/Game/Widgets/W_DialogueBox.SetNewText` (`self.WidgetDialogue`) (`|GetArrayItem` (`self.Dialogue`) (`self.DialogueIndex`)))
  (`UserWidget.AddToViewport` (`self.WidgetDialogue`) 0))

(event `ProgressDialogue`
  (`/Engine/EditorBlueprintResources/StandardMacros.IncrementInt` (`self.DialogueIndex`)
    (:`  `
      (if (>= (`self.DialogueIndex`) (`KismetArrayLibrary.Array_Length` (`self.Dialogue`)))
        (`self.ClearDialogueQueue`)
        (else
          (`self.DisplayNextLine`))))))

(event `ClearDialogueQueue`
  (set `self.DialogueIndex` 0)
  (`KismetArrayLibrary.Array_Clear` (`self.Dialogue`))
  (set `self.IsDisplaying` false)
  (`Widget.RemoveFromParent` (`self.WidgetDialogue`)))

(event `AddDialogueToQueue`
  (params (NewDialogueLine :type Text))
  (`KismetArrayLibrary.Array_Add` (`self.Dialogue`) NewDialogueLine)
  (if (not (`self.IsDisplaying`))
    (`self.DisplayNextLine`)))

(fn `UserConstructionScript`)