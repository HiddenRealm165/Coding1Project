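; BP_Spark is a carryable flame that the player picks up on overlap and holds in the right-hand socket.
; While held, a looping timeline drains player health by the current Intensity, and the primary action spends health to raise Intensity.
; Intensity drives the Niagara fire through a float curve; at its minimum the spark drops, queues a loss dialogue and destroys itself.
; Dropping briefly delays re-enabling physics to avoid flinging.
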(event `self.ReceiveBeginPlay`
  (bind _returnvalue (`GameplayStatics.GetActorOfClass` "/Game/Blueprints/BP_Dialogue_Manager.BP_Dialogue_Manager_C"))
  (set `self.DialogueManager` _returnvalue))

(event `self.ReceiveActorBeginOverlap`
  (params (OtherActor :type "Actor Object Reference"))
  (bind _asbp_third_person_character (cast `/Game/ThirdPerson/Blueprints/BP_ThirdPersonCharacter` OtherActor))
  (bind _output_get (set `self.Player` _asbp_third_person_character))
  (`/Game/ThirdPerson/Blueprints/BP_ThirdPersonCharacter.TryToPickupItem` _output_get self))

(event `self.ReceiveTick`
  (params (DeltaSeconds :type "Float (single-precision)")))

(event `ModifyIntensity`
  (params (`Modify Value` :type "Float (double-precision)"))
  (bind _intensity (`self.Intensity`))
  ; Handling Intensity
  (bind _output_get (set `self.Intensity` (+ (`self.Intensity`) `Modify Value`)))
  (if (<= _output_get (`self.IntensityMinimum`))
    (`self.Spark Lost`)
    (else
      (if (> (`self.Intensity`) (`self.IntensityMaximum`))
        (set `self.Intensity` (`self.IntensityMaximum`)))
      (`NiagaraComponent.SetVariableFloat` (`self.Niagara`) "FireIntensity" (`CurveFloat.GetFloatValue` (`self.FireIntensityCurve`) _intensity))
      (`NiagaraComponent.ReinitializeSystem` (`self.Niagara`))
      (`KismetSystemLibrary.PrintString` (`KismetStringLibrary.Concat_StrStr` "Spark Intensity: " (`KismetStringLibrary.Conv_DoubleToString` _intensity))))))

(event `StartPlayerBurn`
  ; Player Burn Over Time
  (`Timeline|PlayerBurnTimeline` :!label _label
    (:`Finished`
      (`/Game/ThirdPerson/Blueprints/BP_ThirdPersonCharacter.ModifyHealth` (`self.Player`) (* (`self.Intensity`) -1.0))
      (`self.LoopPlayerBurn`))))

(event `LoopPlayerBurn`
  ; Player Burn Over Time
  (goto _label :!via `PlayFromStart`))

(event `Spark Lost`
  ; Handling Intensity
  (`KismetSystemLibrary.PrintString` "Spark Destroyed")
  (`/Game/ThirdPerson/Blueprints/BP_ThirdPersonCharacter.TryToDropItem` (`self.Player`))
  (`/Game/Blueprints/BP_Dialogue_Manager.AddDialogueToQueue` (`self.DialogueManager`) "Your spark was lost. Were you being careful enough? Was it an accident? Sometimes life isn't fair, the mind isn't perfect, ideas fall through. Try to take care of yourself, and cherish the sparks you migth have left.")
  (`self.K2_DestroyActor`))

(event `StopPlayerBurn`
  ; Player Burn Over Time
  (goto _label :!via `Stop`))

(event `/Game/Blueprints/BPI_Item.Pickup`
  ; Player Interaction
  (`KismetSystemLibrary.PrintText` "Spark Picked Up")
  (`PrimitiveComponent.SetSimulatePhysics` (`self.SM_Mesh`) false)
  (`PrimitiveComponent.SetCollisionEnabled` (`self.SM_Mesh`) "NoCollision")
  (`self.K2_AttachToComponent` (`Character.Mesh` (`self.Player`)) "HandGrip_R" "SnapToTarget" "SnapToTarget" "KeepRelative")
  (`self.StartPlayerBurn`))

(event `/Game/Blueprints/BPI_Item.PrimaryAction`
  ; Player Interaction
  (`/Game/ThirdPerson/Blueprints/BP_ThirdPersonCharacter.ModifyHealth` (`self.Player`) (* (`self.PlayerFuelHealthCost`) -1.0))
  (`self.ModifyIntensity` (`self.PlayerFuelIntensityIncrease`)))

(event `/Game/Blueprints/BPI_Item.Drop`
  ; Player Interaction
  (`KismetSystemLibrary.PrintText` "Spark Drop Action")
  (`self.K2_DetachFromActor` "KeepWorld" "KeepWorld" "KeepWorld")
  (`self.StopPlayerBurn`)
  (`KismetSystemLibrary.Delay` 0.1) ; Prevents player's momentum from\nflinging Spark when dropped.
  (`PrimitiveComponent.SetCollisionEnabled` (`self.SM_Mesh`) "QueryAndPhysics")
  (`PrimitiveComponent.SetSimulatePhysics` (`self.SM_Mesh`) true))

(fn `UserConstructionScript`)