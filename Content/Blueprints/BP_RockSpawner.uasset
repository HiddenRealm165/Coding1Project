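; BP_RockSpawner is a rock item the third-person character can carry; despite its name, it shows no spawning logic.
; On overlap it caches the character and calls TryToPickupItem with itself.
; Pickup disables physics and collision on both meshes, then calls attach to the right-hand grip socket.
; Drop detaches and restores both, while PrimaryAction only prints debug text.
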(event `self.ReceiveActorBeginOverlap`
  (params (OtherActor :type "Actor Object Reference"))
  (bind _asbp_third_person_character (cast `/Game/ThirdPerson/Blueprints/BP_ThirdPersonCharacter` OtherActor))
  (bind _output_get (set `self.Player` _asbp_third_person_character))
  (`/Game/ThirdPerson/Blueprints/BP_ThirdPersonCharacter.TryToPickupItem` _output_get self))

(event `/Game/Blueprints/BPI_Item.Pickup`
  (`KismetSystemLibrary.PrintText` "Rock  Picked Up")
  (`PrimitiveComponent.SetSimulatePhysics` (`self.StaticMesh`) false)
  (`PrimitiveComponent.SetCollisionEnabled` (`self.StaticMesh`) "NoCollision")
  (`PrimitiveComponent.SetCollisionEnabled` (`self.StaticMesh1`) "NoCollision")
  (`self.K2_AttachToComponent` (`Character.Mesh` (`self.Player`)) "HandGrip_R" "SnapToTarget" "SnapToTarget" "KeepRelative"))

(event `/Game/Blueprints/BPI_Item.PrimaryAction`
  (`KismetSystemLibrary.PrintText` "Rock Primary Action"))

(event `/Game/Blueprints/BPI_Item.Drop`
  (`KismetSystemLibrary.PrintText` "Rock Drop Action")
  (`self.K2_DetachFromActor` "KeepWorld" "KeepWorld" "KeepWorld")
  (`PrimitiveComponent.SetSimulatePhysics` (`self.StaticMesh`) true)
  (`PrimitiveComponent.SetCollisionEnabled` (`self.StaticMesh`) "QueryAndPhysics")
  (`PrimitiveComponent.SetCollisionEnabled` (`self.StaticMesh1`) "QueryAndPhysics"))

(fn `UserConstructionScript`)