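; BP_SparkRain is an actor that drains the intensity of any BP_Spark overlapping it.
; Begin and end overlap events maintain the Sparks array, and each entering spark calls Play on SparkDrainTimeline.
; Whenever the timeline finishes, it lowers every tracked spark's intensity by SparkDrainAmount and restarts, acting as a repeating timer.
; StopSparkDrain can halt the loop, but nothing in this graph calls it, even when sparks leave.
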(event `self.ReceiveActorBeginOverlap`
  (params (OtherActor :type "Actor Object Reference"))
  (bind _asbp_spark (cast `/Game/Blueprints/BP_Spark` OtherActor))
  (`KismetArrayLibrary.Array_Add` (`self.Sparks`) _asbp_spark)
  (`self.StartSparkDrain`))

(event `self.ReceiveActorEndOverlap`
  (params (OtherActor :type "Actor Object Reference"))
  (for _array_element (`self.Sparks`)
    (if (== _array_element OtherActor)
      (bind _asbp_spark (cast `/Game/Blueprints/BP_Spark` OtherActor))
      (`KismetArrayLibrary.Array_RemoveItem` (`self.Sparks`) _asbp_spark))))

(event `StartSparkDrain`
  (`Timeline|SparkDrainTimeline` :!label _label
    (:`Finished`
      (for _array_element (`self.Sparks`)
        (`/Game/Blueprints/BP_Spark.ModifyIntensity` _array_element (* (`self.SparkDrainAmount`) -1.0)))
      (`self.LoopSparkDrain`))))

(event `LoopSparkDrain`
  (goto _label :!via `PlayFromStart`))

(event `StopSparkDrain`
  (goto _label :!via `Stop`))

(fn `UserConstructionScript`)