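; BP_Door is a locked door that the third-person character opens by spending a key.
; When BP_ThirdPersonCharacter overlaps it with at least one key, it removes a key, then hides the door mesh and box collision and disables their collision.
; The SpawnDoor event restores a hidden door by making both components visible again and re-enabling their collision.
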(event `self.ReceiveActorBeginOverlap`
  (params (OtherActor :type "Actor Object Reference"))
  (bind _asbp_third_person_character (cast `/Game/ThirdPerson/Blueprints/BP_ThirdPersonCharacter` OtherActor))
  (if (> (`/Game/ThirdPerson/Blueprints/BP_ThirdPersonCharacter.TotalKeys` _asbp_third_person_character) 0)
    (`/Game/ThirdPerson/Blueprints/BP_ThirdPersonCharacter.RemoveKey` _asbp_third_person_character)
    (`SceneComponent.SetVisibility` (`self.SM_Door`) false false)
    (`PrimitiveComponent.SetCollisionEnabled` (`self.SM_Door`) "NoCollision")
    (`SceneComponent.SetVisibility` (`self.BoxCollision`) false false)
    (`PrimitiveComponent.SetCollisionEnabled` (`self.BoxCollision`) "NoCollision")))

(event `SpawnDoor`
  (if (not (`SceneComponent.IsVisible` (`self.SM_Door`)))
    (`SceneComponent.SetVisibility` (`self.SM_Door`) true false)
    (`PrimitiveComponent.SetCollisionEnabled` (`self.SM_Door`) "QueryAndPhysics")
    (`SceneComponent.SetVisibility` (`self.BoxCollision`) true false)
    (`PrimitiveComponent.SetCollisionEnabled` (`self.BoxCollision`) "QueryOnly")))

(fn `UserConstructionScript`)